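; BP_Trap is a single-use trap actor that damages a Robber who overlaps it.
; On overlap it type-checks the other actor, stores it as RobberReference, applies damage and destroys itself.
; The skeletal mesh animation check currently leads to identical branches, as the PlayAnimation node is unconnected.
; A loop reading the RequiredMaterials data table for a material check is also unconnected and unfinished.
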(event EventBeginPlay)

(event Collision|EventActorBeginOverlap
  (params (OtherActor :type Actor%20Object%20Reference))
  ;[1 1 1] Ensure Robber triggered it
  (if (Class|GameplayStatics|ObjectIsA OtherActor)
    (Variables|Robber|SetRobber%20Reference OtherActor)
    (if (Class|SkeletalMeshComponent|HasValidAnimationInstance (Variables|Default|GetTrapSkeletalMesh)) ; Check if an animation exists for this trap
      ;[1 1 1] Play Animation then deal damage
      (Game|Damage|ApplyDamage (Variables|Robber|GetRobber%20Reference) 1.0 0 self)
      (Actor|DestroyActor)
      (else
        ;[1 1 1] Deal Damage Directly
        (Game|Damage|ApplyDamage (Variables|Robber|GetRobber%20Reference) 1.0 0 self)
        (Actor|DestroyActor)))))

(event EventTick
  (params (DeltaSeconds :type Float%20%28single-precision%29)))

(fn ConstructionScript)