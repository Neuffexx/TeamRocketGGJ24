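; A WIP player character Blueprint that handles third-person movement, jumping and camera look through Enhanced Input.
; On BeginPlay it adds the IMC_ThirdPerson mapping context for player controller 0.
; Movement follows control rotation, with pitch zeroed for the forward direction.
; Vertical look supports inversion, but yaw input is multiplied by zero, disabling horizontal look and leaving the X-invert selection unconnected.
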(event Input|EnhancedActionEvents|EnhancedInputActionINP_Jump
  (params (ActionValue :type Boolean) (ElapsedSeconds :type Float%20%28double-precision%29) (TriggeredSeconds :type Float%20%28double-precision%29) (InputAction :type Input%20Action%20Object%20Reference :default "/Game/WIP/AlexisDemetriou/INP_Jump.INP_Jump"))
  (:Started
    (Character|Jump))
  (:Completed
    (Character|StopJumping)))

(event Input|EnhancedActionEvents|EnhancedInputActionINP_MoveAround
  (params (ActionValue :type Vector%202D%20Structure) (ElapsedSeconds :type Float%20%28double-precision%29) (TriggeredSeconds :type Float%20%28double-precision%29) (InputAction :type Input%20Action%20Object%20Reference :default "/Game/WIP/AlexisDemetriou/INP_MoveAround.INP_MoveAround"))
  (bind _returnvalue (Pawn|GetControlRotation :!class /Script/Engine.Pawn))
  (:Triggered
    (Pawn|Input|AddMovementInput (Math|Vector|GetRightVector (Pawn|GetControlRotation :!class /Script/Engine.Pawn)) (.x ActionValue) false)
    (Pawn|Input|AddMovementInput (Math|Vector|GetForwardVector (Math|Rotator|MakeRotator (.roll _returnvalue) 0.0 (.yaw _returnvalue))) (.y ActionValue) false)))

(event Input|EnhancedActionEvents|EnhancedInputActionINP_LookAround
  (params (ActionValue :type Vector%202D%20Structure) (ElapsedSeconds :type Float%20%28double-precision%29) (TriggeredSeconds :type Float%20%28double-precision%29) (InputAction :type Input%20Action%20Object%20Reference :default "/Game/WIP/AlexisDemetriou/INP_LookAround.INP_LookAround"))
  (:Triggered
    (Pawn|Input|AddControllerYawInput (* (.x ActionValue) 0.0))
    (Pawn|Input|AddControllerPitchInput (* (.y ActionValue) (Math|Float|SelectFloat -1.0 1.0 (Variables|Default|GetInvertCameraY))))))

(event EventBeginPlay
  (bind _returnvalue (Game|GetPlayerController 0))
  (bind _returnvalue_2 (PlayerController|LocalPlayerSubsystems|GetEnhancedInputLocalPlayerSubsystem _returnvalue))
  (Utilities|IsValid _returnvalue_2
    (:Is%20Valid
      (Input|AddMappingContext _returnvalue_2 "/Game/WIP/AlexisDemetriou/IMC_ThirdPerson.IMC_ThirdPerson" 0 "(bIgnoreAllPressedKeysUntilRelease=True,bForceImmediately=False)"))))

(event Collision|EventActorBeginOverlap
  (params (OtherActor :type Actor%20Object%20Reference)))

(event EventTick
  (params (DeltaSeconds :type Float%20%28single-precision%29)))

(fn ConstructionScript)