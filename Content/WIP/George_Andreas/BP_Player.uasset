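; Player Blueprint in a WIP folder that detects and triggers interactable actors in front of the player.
; Every tick, InteractTrace runs a short sphere trace from the head socket along the camera manager's forward vector, with debug drawing on.
; It caches the hit actor, flags whether it implements BPI_Interact and prints "E" as a prompt.
; Pressing the 1 key sends InteractWithMessage to that actor when interaction is allowed.
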(event EventBeginPlay)

(event Collision|EventActorBeginOverlap
  (params (OtherActor :type Actor%20Object%20Reference)))

(event EventTick
  (params (DeltaSeconds :type Float%20%28single-precision%29))
  (CallFunction|InteractTrace))

(event Input|KeyboardEvents|1
  (params (Key :type Key%20Structure :default "None"))
  (:Pressed
    (if (Variables|Default|GetbCanInteract?)
      (bind _out_hit_hit_actor (Variables|Default|GetOut%20Hit%20Hit%20Actor)
        (:then
          (Class|BPIInteract|Interactwith(Message) _out_hit_hit_actor))
        (:else)))))

(fn ConstructionScript)

(fn InteractTrace
  (bind _mesh (Variables|Character|GetMesh))
  (bind _returnvalue (Transformation|GetSocketLocation _mesh "head"))
  (bind _outhit (Collision|SphereTraceByChannel _returnvalue (+ _returnvalue (* (Transformation|GetActorForwardVector (Game|GetPlayerCameraManager 0)) 1e+02)) 15.0 "TraceTypeQuery1" false 0 "ForDuration"))
  (Variables|Default|SetOut%20Hit%20Hit%20Actor (.hitactor _outhit))
  (if (Utilities|DoesObjectImplementInterface (.hitactor _outhit) "/Game/BlueprintClasses/BPI_Interact.BPI_Interact_C")
    (Variables|Default|SetbCanInteract? true)
    (Development|PrintString "E")
    (else
      (Variables|Default|SetbCanInteract? false))))