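; AI controller that runs the BT_ThiefBehaviour behavior tree and feeds it perception data about the player.
; Perception updates go to HandleSenseSight, which filters for player character stimuli whose sense class equals AISenseConfig_Sight (a config class, not AISense_Sight).
; It sets the Target blackboard key while the player is sensed, otherwise clears it and stores the stimulus position in LastKnownLocation.
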(event OnTargetPerceptionUpdated(AIPerception)
  (params (Actor :type Actor%20Object%20Reference) (Stimulus :type AI%20Stimulus%20Structure))
  (CallFunction|HandleSenseSight Actor Stimulus))

(event EventBeginPlay
  (AI|RunBehaviorTree "/Game/WIP/George_Andreas/BT_ThiefBehaviour.BT_ThiefBehaviour"))

(fn ConstructionScript)

(fn HandleSenseSight
  (params (Actor :type Actor%20Object%20Reference) (Stimulus :type AI%20Stimulus%20Structure))
  (bind _returnvalue (Class|AIPerceptionSystem|GetSenseClassforStimulus Stimulus))
  (if (== _returnvalue "/Script/AIModule.AISenseConfig_Sight")
    (if (== Actor (Game|GetPlayerCharacter 0))
      (AI|Components|Blackboard|SetValueasObject (Variables|Default|GetBlackboard) (Utilities|Name|MakeLiteralName "Target") (Utilities|SelectObject (Game|GetPlayerCharacter 0) 0 (.bsuccessfullysensed Stimulus)))
      (if (not (.bsuccessfullysensed Stimulus))
        (AI|Components|Blackboard|SetValueasVector (Variables|Default|GetBlackboard) (Utilities|Name|MakeLiteralName "LastKnownLocation") (.stimuluslocation Stimulus)))
      (else
        (return)))
    (else
      (return))))